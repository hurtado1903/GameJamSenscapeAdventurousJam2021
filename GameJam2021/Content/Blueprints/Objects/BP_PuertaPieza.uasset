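; A door Blueprint (BP_PuertaPieza) that opens through interaction once the player has done enough actions.
; Interact compares the character's InteractCounter with ActionsToPass, then plays a collapse sound and runs the OpenDoors timeline, which drives the door's yaw.
; The first Box overlap sets HasBeenOpen and, if the actor is BP_CharacterEd, reverses the timeline to close the door.
; DoOnce precedes the cast, so any actor consumes it.
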(event OnComponentBeginOverlap(Box)
  (params (OverlappedComponent :type Primitive%20Component%20Object%20Reference) (OtherActor :type Actor%20Object%20Reference) (OtherComp :type Primitive%20Component%20Object%20Reference) (OtherBodyIndex :type Integer) (bFromSweep :type Boolean) (SweepResult :type Hit%20Result%20Structure%20%28by%20ref%29))
  (Utilities|FlowControl|DoOnce false
    (:Completed
      (Variables|Default|SetHasBeenOpen? true)
      (Utilities|Casting|CastToBP_CharacterEd OtherActor)
      (bind _opendoor (Timeline|OpenDoors Reverse)
        (:Update
          (Transformation|SetRelativeRotation (Variables|Default|GetPuerta) (Math|Rotator|MakeRotator 0.0 0.0 _opendoor) false false))))))

(event Custom|OpenDoor
  (bind _opendoor (Timeline|OpenDoors Play)
    (:Update
      (Transformation|SetRelativeRotation (Variables|Default|GetPuerta) (Math|Rotator|MakeRotator 0.0 0.0 _opendoor) false false))))

(fn ConstructionScript)

(fn FocusObject
  (return false))

(fn InspecObject
  (return false))

(fn Interact
  (bind _asbp_character_ed (Utilities|Casting|CastToBP_CharacterEd (Game|Player|GetPlayerPawn 0)))
  (if (== (Variables|/Game/MetaHumans/Ed/BP_CharacterEd.BP_CharacterEd_C|GetInteractCounter _asbp_character_ed) (Variables|/Game/MetaHumans/Ed/BP_CharacterEd.BP_CharacterEd_C|GetActions%20to%20pass _asbp_character_ed))
    (Audio|PlaySoundatLocation "/Game/StarterContent/Audio/Collapse01.Collapse01" (Transformation|GetActorLocation) "0, 0, 0" 1.0 1.0 0.0 0 0 0)
    (CallFunction|OpenDoor)
    (return false)))