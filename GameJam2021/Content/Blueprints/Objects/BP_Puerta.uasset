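; BP_Puerta is an interactable door that swings open.
; Both Open and Interact trigger the OpenDoor event, which plays the OpenDoors timeline to drive the relative yaw of the Puerta component.
; Interact reports success, while FocusObject and InspecObject simply return false, and no closing logic is present.
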(event Custom|OpenDoor
  (bind _opendoor (Timeline|OpenDoors Play)
    (:Update
      (Transformation|SetRelativeRotation (Variables|Default|GetPuerta) (Math|Rotator|MakeRotator 0.0 0.0 _opendoor) false false))))

(event EventBeginPlay)

(event Collision|EventActorBeginOverlap
  (params (OtherActor :type Actor%20Object%20Reference)))

(event EventTick
  (params (DeltaSeconds :type Float%20%28single-precision%29)))

(fn ConstructionScript)

(fn Open
  (CallFunction|OpenDoor))

(fn FocusObject
  (return false))

(fn InspecObject
  (return false))

(fn Interact
  (CallFunction|OpenDoor)
  (return true))