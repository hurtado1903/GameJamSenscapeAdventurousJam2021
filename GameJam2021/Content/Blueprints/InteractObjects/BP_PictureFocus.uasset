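; BP_PictureFocus is an interactable object, apparently a picture, that responds to being focused on rather than interacted with or inspected.
; The first FocusObject call sets an Interacted flag, plays a pitched-up collapse sound at the actor, runs the parent's InteractSuccess and reports success.
; InspecObject and Interact always return false.
; Logic to increment the character's InteractCounter and destroy the actor is left unconnected.
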(event EventBeginPlay
  (Variables|Default|SetInteracted? false))

(event Collision|EventActorBeginOverlap
  (params (OtherActor :type Actor%20Object%20Reference)))

(event EventTick
  (params (DeltaSeconds :type Float%20%28single-precision%29)))

(fn ConstructionScript
  (|CallParentFunction))

(fn InteractSuccess
  (|CallParentFunction))

(fn FocusObject
  (if (not (Variables|Default|GetInteracted?))
    (bind _output_get (Variables|Default|SetInteracted? true))
    (Audio|PlaySoundatLocation "/Game/StarterContent/Audio/Collapse01.Collapse01" (Transformation|GetActorLocation) "0, 0, 0" 0.8 2.0 0.0 0 0 0)
    (CallFunction|InteractSuccess)
    (return true _output_get)))

(fn InspecObject
  (return false))

(fn Interact
  (return false))