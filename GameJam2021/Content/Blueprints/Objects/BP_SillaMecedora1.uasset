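; Rocking chair actor that rocks through a timeline and can be stopped through focus interaction.
; On BeginPlay, the Estado enum plays or reverses the Mecer timeline, whose updates scale Rotacion into the actor's relative rotation and set Estado from playback direction.
; FocusObject stops the timeline, prints a debug string and signals interaction success.
; Interact only returns true, InspecObject returns false, and sphere overlap events are empty.
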(event OnComponentBeginOverlap(Sphere)
  (params (OverlappedComponent :type Primitive%20Component%20Object%20Reference) (OtherActor :type Actor%20Object%20Reference) (OtherComp :type Primitive%20Component%20Object%20Reference) (OtherBodyIndex :type Integer) (bFromSweep :type Boolean) (SweepResult :type Hit%20Result%20Structure%20%28by%20ref%29)))

(event OnComponentEndOverlap(Sphere)
  (params (OverlappedComponent :type Primitive%20Component%20Object%20Reference) (OtherActor :type Actor%20Object%20Reference) (OtherComp :type Primitive%20Component%20Object%20Reference) (OtherBodyIndex :type Integer)))

(event EventBeginPlay
  (switch Utilities|FlowControl|Switch|SwitchonEN_Movimiento (Variables|Default|GetEstado)
    (:NewEnumerator0
      (bind (_direction _mecer) (Timeline|Mecer Play)
        (:Update
          (Transformation|SetActorRelativeRotation (* (Variables|Default|GetRotacion) _mecer))
          (if (Utilities|Enum|Equal(Enum) _direction "Forward")
            (Variables|Default|SetEstado "NewEnumerator0")
            (else
              (Variables|Default|SetEstado "NewEnumerator1")))
          (if (Utilities|Enum|Equal(Enum) (Variables|Default|GetEstado) "NewEnumerator2")
            (Timeline|Mecer Stop)))))
    (:NewEnumerator1
      (Timeline|Mecer Reverse))))

(fn ConstructionScript)

(fn FocusObject
  (Audio|Components|Audio|Stop (Variables|Default|GetMecer))
  (Development|PrintString "Hello")
  (CallFunction|InteractSuccess)
  (return true))

(fn InspecObject
  (return false))

(fn Interact
  (return true))