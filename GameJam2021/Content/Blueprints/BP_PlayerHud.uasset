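; BP_PlayerHud manages the player's on-screen UI, switching between the GameHud and Instrucciones widgets.
; On BeginPlay it creates both widgets for player 0 and adds them to the viewport together.
; The MostrarHud input action drives a FlipFlop that removes all widgets, then adds a newly created Instrucciones or GameHud on alternate presses, starting with Instrucciones.
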(event EventBeginPlay
  (bind _returnvalue (Game|GetPlayerController 0))
  (bind _returnvalue_2 (UserInterface|CreateWidget "/Game/WidgetsUi/GameHud.GameHud_C" _returnvalue))
  (UserInterface|Viewport|AddtoViewport _returnvalue_2 0)
  (bind _returnvalue_3 (UserInterface|CreateWidget "/Game/WidgetsUi/Instrucciones.Instrucciones_C" _returnvalue))
  (UserInterface|Viewport|AddtoViewport _returnvalue_3 0))

(event Input|ActionEvents|InputActionMostrarHud
  (params (Key :type Key%20Structure :default "None"))
  (:Pressed
    (Utilities|FlowControl|FlipFlop
      (:A
        (Viewport|RemoveAllWidgets)
        (bind _returnvalue (UserInterface|CreateWidget "/Game/WidgetsUi/Instrucciones.Instrucciones_C" (Game|GetPlayerController 0)))
        (UserInterface|Viewport|AddtoViewport _returnvalue 0))
      (:B
        (Viewport|RemoveAllWidgets)
        (bind _returnvalue_2 (UserInterface|CreateWidget "/Game/WidgetsUi/GameHud.GameHud_C" (Game|GetPlayerController 0)))
        (UserInterface|Viewport|AddtoViewport _returnvalue_2 0)))))

(fn ConstructionScript)