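; BP_Bolsa is an interactable bag object that responds once when focused.
; The first FocusObject call sets the Interacted flag, plays a soft bag sound at the actor's location, calls InteractSuccess and returns success.
; InspecObject and Interact both return false, so focus is the only active interaction.
; The event graph is unused, and the construction script only calls the parent's.
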(event EventBeginPlay)

(event Collision|EventActorBeginOverlap
  (params (OtherActor :type Actor%20Object%20Reference)))

(event EventTick
  (params (DeltaSeconds :type Float%20%28single-precision%29)))

(fn ConstructionScript
  (|CallParentFunction))

(fn FocusObject
  (if (not (Variables|Default|GetInteracted?))
    (bind _output_get (Variables|Default|SetInteracted? true))
    (Audio|PlaySoundatLocation "/Game/Sonidos/Props/Cues/bolsa_suave_Cue.bolsa_suave_Cue" (Transformation|GetActorLocation) "0, 0, 0" 1.0 1.0 0.0 0 0 0)
    (CallFunction|InteractSuccess)
    (return true _output_get)))

(fn InspecObject
  (return false))

(fn Interact
  (return false))