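; BP_ActorInteractParent is, by its name, a parent actor for interactable objects, and it clears its Interacted flag on BeginPlay.
; InteractSuccess increments InteractCounter on the player's BP_CharacterEd, prints the count and returns false, without setting Interacted.
; SetupOutlineMesh does nothing, as its nodes for copying the object's mesh and applying M_MeshOutline to each material slot are disconnected.
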(event EventBeginPlay
  (Variables|Default|SetInteracted? false))

(fn ConstructionScript)

(fn InteractSuccess
  (bind _asbp_character_ed (Utilities|Casting|CastToBP_CharacterEd (Game|GetPlayerCharacter 0)))
  (bind _output_get (Variables|/Game/MetaHumans/Ed/BP_CharacterEd.BP_CharacterEd_C|SetInteractCounter _asbp_character_ed (+ (Variables|/Game/MetaHumans/Ed/BP_CharacterEd.BP_CharacterEd_C|GetInteractCounter _asbp_character_ed) 1)))
  (Development|PrintString (Utilities|String|ToString(Integer) _output_get))
  (return false))

(fn SetupOutlineMesh)