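; BP_SillaMecedora is an interactable rocking chair that rocks until the player focuses on it.
; On BeginPlay, an Estado enum plays or reverses the Mecer timeline, whose curve scales Rotacion into the mesh's relative rotation.
; Timeline updates set Estado from the playback direction.
; FocusObject stops the timeline, prints a debug message and reports success, while InspecObject and Interact just return false.
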(event EventBeginPlay
  (switch Utilities|FlowControl|Switch|SwitchonEN_Movimiento (Variables|Default|GetEstado)
    (:NewEnumerator0
      (bind (_direction _mecer) (Timeline|Mecer Play)
        (:Update
          (Transformation|SetRelativeRotation (Variables|Default|GetStaticMesh) (* (Variables|Default|GetRotacion) _mecer) false false)
          (if (Utilities|Enum|Equal(Enum) _direction "Forward")
            (Variables|Default|SetEstado "NewEnumerator0")
            (else
              (Variables|Default|SetEstado "NewEnumerator1")))
          (if (Utilities|Enum|Equal(Enum) (Variables|Default|GetEstado) "NewEnumerator2")
            (Timeline|Mecer Stop)))))
    (:NewEnumerator1
      (Timeline|Mecer Reverse))))

(fn ConstructionScript
  (|CallParentFunction))

(fn FocusObject
  (Audio|Components|Audio|Stop (Variables|Default|GetMEcer))
  (Development|PrintString "Hello")
  (CallFunction|InteractSuccess)
  (return true))

(fn InspecObject
  (return false))

(fn Interact
  (return false))