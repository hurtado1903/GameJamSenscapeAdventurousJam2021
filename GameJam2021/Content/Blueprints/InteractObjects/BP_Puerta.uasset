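; BP_Puerta is an interactable one-way door that swings open on Interact and shuts behind the player.
; Interact calls OpenDoor until HasBeenOpen is set; a DoOnce there plays the sound and a yaw timeline.
; BP_CharacterEd overlapping the Box, or the Close event, runs CloseDoor and reverses the timeline.
; CloseDoor sets HasBeenOpen, turns the light red and plays the closing sound, blocking further interaction.
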(event OnComponentBeginOverlap(Box)
  (params (OverlappedComponent :type Primitive%20Component%20Object%20Reference) (OtherActor :type Actor%20Object%20Reference) (OtherComp :type Primitive%20Component%20Object%20Reference) (OtherBodyIndex :type Integer) (bFromSweep :type Boolean) (SweepResult :type Hit%20Result%20Structure%20%28by%20ref%29))
  (Utilities|Casting|CastToBP_CharacterEd OtherActor)
  (CallFunction|CloseDoor)
  (bind _opendoor (Timeline|OpenDoors Reverse)
    (:Update
      (Transformation|SetRelativeRotation (Variables|Default|GetPuerta) (Math|Rotator|MakeRotator 0.0 0.0 _opendoor) false false))))

(event Custom|OpenDoor
  (Utilities|FlowControl|DoOnce false
    (:Completed
      (Audio|PlaySoundatLocation "/Game/Sonidos/Props/Cues/Puerta_abrir.Puerta_abrir" (Transformation|GetActorLocation) "0, 0, 0" 1.0 1.0 0.0 0 0 0)
      (bind _opendoor (Timeline|OpenDoors Play)
        (:Update
          (Transformation|SetRelativeRotation (Variables|Default|GetPuerta) (Math|Rotator|MakeRotator 0.0 0.0 _opendoor) false false))))))

(event Custom|Close
  (CallFunction|CloseDoor)
  (bind _opendoor (Timeline|OpenDoors Reverse)
    (:Update
      (Transformation|SetRelativeRotation (Variables|Default|GetPuerta) (Math|Rotator|MakeRotator 0.0 0.0 _opendoor) false false))))

(fn ConstructionScript)

(fn CloseDoor
  (Utilities|FlowControl|DoOnce false
    (:Completed
      (Variables|Default|SetHasBeenOpen? true)
      (Rendering|Components|Light|SetLightColor (Variables|Default|GetPointLight) (Class|KismetMathLibrary|LinearColorRed) true)
      (Audio|PlaySoundatLocation "/Game/Sonidos/Props/Cues/Puerta_Cerrar.Puerta_Cerrar" (Transformation|GetActorLocation) "0, 0, 0" 1.0 1.0 0.0 0 0 0))))

(fn FocusObject
  (return false false))

(fn InspecObject
  (return false))

(fn Interact
  (if (not (Variables|Default|GetHasBeenOpen?))
    (CallFunction|OpenDoor)
    (return true)))