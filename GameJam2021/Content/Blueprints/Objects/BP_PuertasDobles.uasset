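; Interactable door Blueprint that swings open when used and closes when the character enters its trigger box.
; Interact calls Open, which plays a sound and runs a timeline that drives the static mesh's yaw.
; Overlap of the box by BP_CharacterEd plays a closing sound and reverses the timeline, with an Open flag guarding both transitions.
; FocusObject and InspecObject are stubs that return false.
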(event OnComponentBeginOverlap(Box)
  (params (OverlappedComponent :type Primitive%20Component%20Object%20Reference) (OtherActor :type Actor%20Object%20Reference) (OtherComp :type Primitive%20Component%20Object%20Reference) (OtherBodyIndex :type Integer) (bFromSweep :type Boolean) (SweepResult :type Hit%20Result%20Structure%20%28by%20ref%29))
  (Utilities|Casting|CastToBP_CharacterEd OtherActor)
  (if (Variables|Default|GetOpen?)
    (Variables|Default|SetOpen? false)
    (Audio|PlaySoundatLocation "/Game/Sonidos/Props/Cues/Puerta_Cerrar.Puerta_Cerrar" (Transformation|GetActorLocation) "0, 0, 0" 1.0 1.0 0.0 0 0 0)
    (bind _rotation (Timeline|OpenDoor Reverse)
      (:Update
        (Transformation|SetRelativeRotation (Variables|Default|GetStaticMesh) (Math|Rotator|MakeRotator 0.0 0.0 _rotation) false false)))))

(event Custom|Open
  (if (not (Variables|Default|GetOpen?))
    (Variables|Default|SetOpen? true)
    (Audio|PlaySoundatLocation "/Game/Sonidos/Props/Cues/Puerta_abrir.Puerta_abrir" (Transformation|GetActorLocation) "0, 0, 0" 1.0 1.0 0.0 0 0 0)
    (bind _rotation (Timeline|OpenDoor Play)
      (:Update
        (Transformation|SetRelativeRotation (Variables|Default|GetStaticMesh) (Math|Rotator|MakeRotator 0.0 0.0 _rotation) false false)))))

(event EventBeginPlay)

(event Collision|EventActorBeginOverlap
  (params (OtherActor :type Actor%20Object%20Reference)))

(event EventTick
  (params (DeltaSeconds :type Float%20%28single-precision%29)))

(fn ConstructionScript)

(fn FocusObject
  (return false false))

(fn InspecObject
  (return false))

(fn Interact
  (CallFunction|Open)
  (return true))