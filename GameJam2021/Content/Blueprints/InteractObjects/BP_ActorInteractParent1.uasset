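; Base interactable actor, by its name a parent class, that tracks whether it has been interacted with and starts uninteracted.
; FocusObject calls InteractSuccess, which increments InteractCounter on BP_CharacterEd with debug prints, then sets and returns Interacted as true.
; Interact and InspecObject are stubs returning false.
; SetupOutlineMesh is empty, with disconnected logic for copying the object's mesh to an outline component using M_MeshOutline.
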(event EventBeginPlay
  (Variables|Default|SetInteracted? false))

(fn ConstructionScript)

(fn InteractSuccess
  (bind _asbp_character_ed (Utilities|Casting|CastToBP_CharacterEd (Game|GetPlayerCharacter 0))
    (:then
      (bind _output_get (Variables|/Game/MetaHumans/Ed/BP_CharacterEd.BP_CharacterEd_C|SetInteractCounter _asbp_character_ed (+ (Variables|/Game/MetaHumans/Ed/BP_CharacterEd.BP_CharacterEd_C|GetInteractCounter _asbp_character_ed) 1)))
      (Development|PrintString (Utilities|String|ToString(Integer) _output_get))
      (return true))
    (:CastFailed
      (Development|PrintString "Hello"))))

(fn SetupOutlineMesh)

(fn FocusObject
  (Development|PrintString "Hello")
  (CallFunction|InteractSuccess)
  (bind _output_get (Variables|Default|SetInteracted? true))
  (return _output_get))

(fn InspecObject
  (return false))

(fn Interact
  (return false))